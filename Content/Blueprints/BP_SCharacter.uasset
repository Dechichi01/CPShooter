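; BP_SCharacter is a character Blueprint that arms itself with a rifle and shows a crosshair.
; On BeginPlay it spawns BP_SRifle, stores it as Weapon, attaches it to the mesh's WeaponSocket and sets itself as owner.
; It also creates the WBP_CrossHair widget and adds it to the viewport.
; A hard-bound left mouse press calls Fire on the weapon, while Tick and the construction script are empty.
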(event EventBeginPlay
  (bind _returnvalue (Game|SpawnActorfromClass "/Game/Blueprints/BP_SRifle.BP_SRifle_C" (Math|Transform|MakeTransform "0, 0, 0") "AlwaysSpawn" 0 0))
  (bind _output_get (Variables|Default|SetWeapon _returnvalue))
  (Transformation|AttachComponentToComponent _output_get (Variables|Character|GetMesh) "WeaponSocket" "SnapToTarget" "SnapToTarget" "SnapToTarget" true)
  (Actor|SetOwner (Variables|Default|GetWeapon) self)
  (bind _returnvalue_2 (UserInterface|CreateWidget "/Game/UI/WBP_CrossHair.WBP_CrossHair_C"))
  (UserInterface|Viewport|AddtoViewport _returnvalue_2 0))

(event EventTick
  (params (DeltaSeconds :type Float%20%28single-precision%29)))

(event Input|MouseEvents|LeftMouseButton
  (params (Key :type Key%20Structure))
  (:Pressed
    (Class|SWeapon|Fire (Variables|Default|GetWeapon))))

(fn ConstructionScript)